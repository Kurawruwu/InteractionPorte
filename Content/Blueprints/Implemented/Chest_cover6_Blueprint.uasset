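; Chest lid Blueprint that opens once the player has used both of two keys on it.
; On Interaction, each key flag held by BP_FirstPersonCharacter triggers, once, a dummy key mesh spawned at runtime, attached to the lid and turned by a Timeline.
; When each turn finishes it sets a flag and calls OpeningChestEvent, which plays a one-time Timeline rotating the lid open when both flags are set.
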(event Custom|OpeningChestEvent
  (if (and (Variables|Default|GetRotateKey1) (Variables|Default|GetRotateKey2))
    (Utilities|FlowControl|DoOnce false
      (:Completed
        (bind _angle (Timeline|OpeningChest Play)
          (:Update
            (Transformation|SetRelativeRotation (Variables|Default|GetChest_cover6_StaticMeshComponent0) (Math|Rotator|MakeRotator (* _angle (Variables|Default|GetAngle)) 0.0 0.0) false false)))))))

(event EventInteraction
  (bind _asbp_first_person_character (Utilities|Casting|CastToBP_FirstPersonCharacter (Game|GetPlayerCharacter 0)))
  (Utilities|FlowControl|Sequence
    (:then_0
      (if (Variables|/Game/Blueprints/Implemented/BP_FirstPersonCharacter.BP_FirstPersonCharacter_C|GetKey1 _asbp_first_person_character)
        (Utilities|FlowControl|DoOnce false
          (:Completed
            (bind _returnvalue (AddComponent|AddStaticMeshComponent false (Math|Transform|MakeTransform "-20.000000,44.000000,58.000000" "-90.000000,0.000000,-180.000000" "1.000000,1.000000,1.000000")))
            (bind _output_get (Variables|Default|SetDummyKey1 _returnvalue))
            (Transformation|AttachComponentToComponent _output_get (Variables|Default|GetChest_cover6_StaticMeshComponent0) "None" "KeepWorld" "KeepWorld" "KeepRelative" true)
            (Collision|SetCollisionEnabled _output_get "NoCollision")
            (bind _newtrack_0 (Timeline|Timeline Play)
              (:Update
                (Transformation|SetRelativeRotation (Variables|Default|GetDummyKey1) (Math|Rotator|MakeRotator 1.8e+02 (Math|Float|Lerp -9e+01 9e+01 _newtrack_0) 0.0) false false))
              (:Finished
                (Variables|Default|SetRotateKey1 true)
                (CallFunction|OpeningChestEvent)))))))
    (:then_1
      (if (Variables|/Game/Blueprints/Implemented/BP_FirstPersonCharacter.BP_FirstPersonCharacter_C|GetKey2 _asbp_first_person_character)
        (Utilities|FlowControl|DoOnce false
          (:Completed
            (bind _returnvalue_2 (AddComponent|AddStaticMeshComponent false (Math|Transform|MakeTransform "20.000000,44.000000,58.000000" "-90.000000,0.000000,-180.000000" "1.000000,1.000000,1.000000")))
            (bind _output_get_2 (Variables|Default|SetDummyKey2 _returnvalue_2))
            (Transformation|AttachComponentToComponent _output_get_2 (Variables|Default|GetChest_cover6_StaticMeshComponent0) "None" "KeepWorld" "KeepWorld" "KeepRelative" true)
            (Collision|SetCollisionEnabled _output_get_2 "NoCollision")
            (bind _newtrack_0_2 (Timeline|Timeline_0 Play)
              (:Update
                (Transformation|SetRelativeRotation (Variables|Default|GetDummyKey2) (Math|Rotator|MakeRotator 1.8e+02 (Math|Float|Lerp -9e+01 9e+01 _newtrack_0_2) 0.0) false false))
              (:Finished
                (Variables|Default|SetRotateKey2 true)
                (CallFunction|OpeningChestEvent)))))))))

(fn ConstructionScript)